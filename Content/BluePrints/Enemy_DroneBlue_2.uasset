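; Blue drone enemy that roams between preset points, fires at the player and is destroyed by any overlap with its box.
; Every few seconds it picks one of four move-location components and a random yaw spin, applied on Tick.
; A self-renewing timer lerps the mesh a small fraction toward the target, easing its arrival.
; A delayed loop snaps the mesh to face the player and spawns a projectile from the arrow.
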(event `self.ReceiveBeginPlay`
  (`self.FindNewLocation`)
  (`self.ShootAtPlayer` :!label _label)
  (`KismetSystemLibrary.Delay` (`KismetMathLibrary.RandomFloatInRange` 3.0 5.0))
  (goto _label))

(event `Moving`
  (bind _skeletalmesh (`self.SkeletalMesh`))
  (set `self.Alpha` 0.0)
  (`KismetSystemLibrary.K2_SetTimerDelegate` (delegate `Moving`) 0.02)
  (set `self.Alpha` (+ (`self.Alpha`) 0.02))
  (`SceneComponent.K2_SetWorldLocation` _skeletalmesh (`KismetMathLibrary.VLerp` (`SceneComponent.K2_GetComponentLocation` _skeletalmesh) (`self.LocationToMove`) (`self.Alpha`)) false false))

(event `self.ReceiveTick`
  (params (DeltaSeconds :type "Float (single-precision)"))
  (`SceneComponent.K2_AddLocalRotation` (`self.SkeletalMesh`) (`KismetMathLibrary.MakeRotator` 0.0 0.0 (`self.Delta Rotation Z (Yaw)`)) false false))

(event `FindNewLocation`
  (bind _array (`|MakeArray` (`self.MoveLocation2`) (`self.MoveLocation1`) (`self.MoveLocation3`) (`self.MoveLocation4`)))
  (set `self.Delta Rotation Z (Yaw)` (`KismetMathLibrary.RandomFloatInRange` -1.0 1.0))
  (set `self.LocationToMove` (`SceneComponent.K2_GetComponentLocation` (`|GetArrayItem` _array (`KismetMathLibrary.RandomIntegerInRange` 0 (`KismetArrayLibrary.Array_LastIndex` _array)))))
  (`self.Moving`)
  (`KismetSystemLibrary.Delay` (`KismetMathLibrary.RandomFloatInRange` 2.0 3.0))
  (`self.FindNewLocation`))

(event `ShootAtPlayer`
  (bind _skeletalmesh (`self.SkeletalMesh`))
  (`SceneComponent.K2_SetWorldRotation` _skeletalmesh (`KismetMathLibrary.FindLookAtRotation` (`SceneComponent.K2_GetComponentLocation` _skeletalmesh) (`SceneComponent.K2_GetComponentLocation` (`Actor.RootComponent` (`GameplayStatics.GetPlayerPawn` 0)))) false false)
  (`|SpawnActorFromClass` "/Game/BluePrints/EnemyProjectile.EnemyProjectile_C" (`SceneComponent.K2_GetComponentToWorld` (`self.Arrow`)) "Undefined" "OverrideRootScale" null null))

(event `self.Box.OnComponentBeginOverlap`
  (params (OverlappedComponent :type "PrimitiveComponent Object Reference") (OtherActor :type "Actor Object Reference") (OtherComp :type "PrimitiveComponent Object Reference") (OtherBodyIndex :type Integer) (bFromSweep :type Boolean) (SweepResult :type "HitResult Structure (by ref)"))
  (`self.K2_DestroyActor`))

(fn `UserConstructionScript`)