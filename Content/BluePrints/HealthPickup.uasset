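; Health pickup actor that gives health to a PitcherCharacter or ConstructionBotCharacter that touches it.
; On overlap it casts the other actor to each character class, calls that class's GainHealth and destroys itself.
; Tick spins the Cube in yaw by a fixed per-frame step.
; AddHealth is empty, and disconnected look-at and HealthProjectile spawn nodes never run.
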(event `self.ReceiveActorBeginOverlap`
  (params (OtherActor :type "Actor Object Reference"))
  (`|ExecutionSequence`
    (:`then_0`
      (bind _aspitcher_character (cast `/Game/FirstPersonBP/Blueprints/PitcherCharacter` OtherActor))
      (`/Game/FirstPersonBP/Blueprints/PitcherCharacter.GainHealth` _aspitcher_character))
    (:`then_1`
      (bind _asconstruction_bot_character (cast `/Game/FirstPersonBP/Blueprints/ConstructionBotCharacter` OtherActor))
      (`/Game/FirstPersonBP/Blueprints/ConstructionBotCharacter.GainHealth` _asconstruction_bot_character)))
  (`self.K2_DestroyActor`))

(event `AddHealth`)

(event `self.ReceiveTick`
  (params (DeltaSeconds :type "Float (single-precision)"))
  (`SceneComponent.K2_AddLocalRotation` (`self.Cube`) (`KismetMathLibrary.MakeRotator` 0.0 0.0 1.0) false false))

(fn `UserConstructionScript`)