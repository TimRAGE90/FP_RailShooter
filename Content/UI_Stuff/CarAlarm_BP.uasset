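; CarAlarm_BP is an actor that flashes a point light and a spot light, apparently as the visual effect of a car alarm.
; On BeginPlay, a Sequence starts two endless Delay loops, one per light, that switch intensity between on and zero.
; Both loops share the same interval, so the lights blink in step, with the spot light set far brighter.
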(event `self.ReceiveBeginPlay`
  (bind _pointlight (`self.PointLight`))
  (bind _spotlight (`self.SpotLight`))
  (`|ExecutionSequence`
    (:`then_0`
      (`LightComponent.SetIntensity` _pointlight 75.0 :!label _label)
      (`KismetSystemLibrary.Delay` 1.25)
      (`LightComponent.SetIntensity` _pointlight 0.0)
      (`KismetSystemLibrary.Delay` 1.25)
      (goto _label))
    (:`then_1`
      (`LightComponent.SetIntensity` _spotlight 100000.0 :!label _label_2)
      (`KismetSystemLibrary.Delay` 1.25)
      (`LightComponent.SetIntensity` _spotlight 0.0)
      (`KismetSystemLibrary.Delay` 1.25)
      (goto _label_2))))

(fn `UserConstructionScript`)